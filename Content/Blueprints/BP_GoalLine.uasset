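; BP_GoalLine is a goal detector that scores when anything finishes overlapping Box3.
; It increments Score1P on player index 1's BP_BallPawn and disables Box3's collision for two seconds to limit repeat triggers.
; The Goal flag is set true just before its check, so it gates nothing.
; Box, Box1 and Box2 only print "No Goal!" on begin overlap.
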(event `self.Box3.OnComponentEndOverlap`
  (params (OverlappedComponent :type "PrimitiveComponent Object Reference") (OtherActor :type "Actor Object Reference") (OtherComp :type "PrimitiveComponent Object Reference") (OtherBodyIndex :type Integer))
  (`|ExecutionSequence`
    (:`then_0`
      (`KismetSystemLibrary.PrintString` "Goal")
      (`PrimitiveComponent.SetCollisionEnabled` (`self.Box3`) "NoCollision")
      (`KismetSystemLibrary.Delay` 2.0)
      (`PrimitiveComponent.SetCollisionEnabled` (`self.Box3`) "QueryAndPhysics"))
    (:`then_1`
      (bind _output_get (set `self.Goal` true))
      (if _output_get
        (bind _asbp_ball_pawn (cast `/Game/Blueprints/BP_BallPawn` (`GameplayStatics.GetPlayerPawn` 1))
          (:`then`
            (set `BallPawn.Score_1P` (+ (`BallPawn.Score_1P` _asbp_ball_pawn) 1) _asbp_ball_pawn)
            (set `self.Goal` false))
          (:`CastFailed`
            (`KismetSystemLibrary.PrintString` "Hello")))
        (else
          (`KismetSystemLibrary.PrintString` "NOOOOOO"))))))

(event `self.Box.OnComponentBeginOverlap`
  (params (OverlappedComponent :type "PrimitiveComponent Object Reference") (OtherActor :type "Actor Object Reference") (OtherComp :type "PrimitiveComponent Object Reference") (OtherBodyIndex :type Integer) (bFromSweep :type Boolean) (SweepResult :type "HitResult Structure (by ref)"))
  (`KismetSystemLibrary.PrintString` "No Goal!" :!label _label))

(event `self.Box1.OnComponentBeginOverlap`
  (params (OverlappedComponent :type "PrimitiveComponent Object Reference") (OtherActor :type "Actor Object Reference") (OtherComp :type "PrimitiveComponent Object Reference") (OtherBodyIndex :type Integer) (bFromSweep :type Boolean) (SweepResult :type "HitResult Structure (by ref)"))
  (goto _label))

(event `self.Box2.OnComponentBeginOverlap`
  (params (OverlappedComponent :type "PrimitiveComponent Object Reference") (OtherActor :type "Actor Object Reference") (OtherComp :type "PrimitiveComponent Object Reference") (OtherBodyIndex :type Integer) (bFromSweep :type Boolean) (SweepResult :type "HitResult Structure (by ref)"))
  (goto _label))

(fn `UserConstructionScript`)